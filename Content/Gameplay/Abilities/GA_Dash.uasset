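; Gameplay ability that dashes the third-person character along its normalized pending movement input.
; On commit it applies GE_Dash, zeroes movement and sends the direction to the character's server event, with locally controlled characters also applying dash velocity immediately.
; Client movement error correction is suspended until the ability ends after a short delay.
; GE_Dash removal sits in a separate ApplyDashVelocity event that this graph never calls.
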(event Custom|ApplyDashVelocity
  (params (LaunchVelocity :type Vector))
  (Utilities|FlowControl|Delay 0.15)
  (Ability|RemoveGameplayEffectFromOwnerWithHandle (Variables|Default|GetDashEffect))
  (Ability|RemoveGameplayEffectFromOwnerWithHandle (Variables|Default|GetDashEffect))
  (Utilities|FlowControl|Delay 0.2)
  (bind _movecomponent (Variables|Default|GetMoveComponent)
    (:then
      (Variables|/Script/Engine.CharacterMovementComponent|SetbIgnoreClientMovementErrorChecksAndCorrection _movecomponent false))
    (:else
      _))
  (Ability|EndAbility))

(event Ability|EventActivateAbility
  (bind _returnvalue (Ability|GetAvatarActorfromActorInfo))
  (bind _asbp_third_person_character (Utilities|Casting|CastToBP_ThirdPersonCharacter _returnvalue))
  (bind _charactermovement (Variables|/Script/Engine.Character|GetCharacterMovement _asbp_third_person_character))
  (bind _returnvalue_2 (Class|PawnMovementComponent|GetPendingInputVector _charactermovement))
  (bind _returnvalue_3 (Math|Vector|Normalize _returnvalue_2))
  (CallFunction|PopulateVars)
  (bind _returnvalue_4 (Ability|CommitAbility))
  (if _returnvalue_4
    (bind _returnvalue_5 (Ability|ApplyGameplayEffectToOwner "/Game/Gameplay/Effects/GE_Dash.GE_Dash_C"))
    (Variables|Default|SetDashEffect _returnvalue_5)
    (bind _movecomponent (Variables|Default|GetMoveComponent)
      (:then
        (Variables|/Script/Engine.CharacterMovementComponent|SetbIgnoreClientMovementErrorChecksAndCorrection _movecomponent true))
      (:else
        _))
    (bind _movecomponent_2 (Variables|Default|GetMoveComponent)
      (:then
        (Pawn|Components|CharacterMovement|ClearAccumulatedForces _movecomponent_2)
        (Variables|/Script/Engine.MovementComponent|SetVelocity _movecomponent_2 "0, 0, 0"))
      (:else
        _))
    (bind _as_character (Variables|Default|GetAs%20Character)
      (:then
        (Default|SERVERApplyDashInput (.AsBP%20Third%20Person%20Character (Utilities|Casting|CastToBP_ThirdPersonCharacter _as_character)) _returnvalue_3)
        (if (Pawn|IsLocallyControlled (.AsBP%20Third%20Person%20Character (Utilities|Casting|CastToBP_ThirdPersonCharacter _as_character)))
          (Default|ApplyDashVelocity (.AsBP%20Third%20Person%20Character (Utilities|Casting|CastToBP_ThirdPersonCharacter _as_character)) (* _returnvalue_3 3e+03))))
      (:else
        _))
    (Utilities|FlowControl|Delay 0.15)
    (bind _movecomponent_3 (Variables|Default|GetMoveComponent)
      (:then
        (Variables|/Script/Engine.CharacterMovementComponent|SetbIgnoreClientMovementErrorChecksAndCorrection _movecomponent_3 false))
      (:else
        _))
    (Ability|EndAbility)))

(event Ability|EventOnEndAbility
  (params (bWasCancelled :type Boolean)))

(fn PopulateVars
  (bind _returnvalue (Ability|GetAvatarActorfromActorInfo))
  (bind _aspawn (Utilities|Casting|CastToPawn _returnvalue))
  (Variables|Default|GetMoveComponent
    (:then
      _)
    (:else
      (Variables|Default|SetMoveComponent (Actor|GetComponentbyClass _returnvalue "/Script/Engine.CharacterMovementComponent"))))
  (Variables|Default|GetController
    (:then
      _)
    (:else
      (Variables|Default|SetController (Pawn|GetController _aspawn))))
  (Variables|Default|GetAs%20Character
    (:then
      _)
    (:else
      (Variables|Default|SetAs%20Character (.AsCharacter (Utilities|Casting|CastToCharacter _aspawn)))))
  (return))