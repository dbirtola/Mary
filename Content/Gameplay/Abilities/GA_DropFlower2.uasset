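; GA_DropFlower2 is a gameplay ability that, despite its name, performs a short forward dash on the avatar character.
; It commits, applies GE_Dash, clears movement forces and launches the character along its forward vector.
; After a brief delay it resets velocity to max speed, removes the effect, then waits before ending.
; Client movement error checks are ignored throughout; input-lock, impulse and authority-check nodes are left disconnected.
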(event Ability|EventActivateAbility
  (bind _returnvalue (Ability|GetAvatarActorfromActorInfo))
  (bind _returnvalue_2 (Ability|GetAvatarActorfromActorInfo))
  (bind _returnvalue_3 (Transformation|GetActorForwardVector _returnvalue_2))
  (bind _aspawn (Utilities|Casting|CastToPawn _returnvalue))
  (Variables|Default|SetMoveComponent (Actor|GetComponentbyClass _returnvalue "/Script/Engine.CharacterMovementComponent"))
  (Variables|Default|SetController (Pawn|GetController _aspawn))
  (Variables|Default|SetAs%20Character (.AsCharacter (Utilities|Casting|CastToCharacter _aspawn)))
  (Ability|CommitAbility)
  (bind _returnvalue_4 (Ability|ApplyGameplayEffectToOwner "/Game/Gameplay/Effects/GE_Dash.GE_Dash_C"))
  (Variables|Default|SetDashEffect _returnvalue_4)
  (Variables|/Script/Engine.CharacterMovementComponent|SetbIgnoreClientMovementErrorChecksAndCorrection (Variables|Default|GetMoveComponent) true)
  (Pawn|Components|CharacterMovement|ClearAccumulatedForces (Variables|Default|GetMoveComponent))
  (Variables|/Script/Engine.MovementComponent|SetVelocity (Variables|Default|GetMoveComponent) "0, 0, 0")
  (Character|LaunchCharacter (Variables|Default|GetAs%20Character) (* _returnvalue_3 1.5e+03) true false)
  (Utilities|FlowControl|Delay 0.15)
  (Variables|/Script/Engine.MovementComponent|SetVelocity (Variables|Default|GetMoveComponent) (* (Class|MovementComponent|GetMaxSpeed (Variables|Default|GetMoveComponent)) _returnvalue_3))
  (Ability|RemoveGameplayEffectFromOwnerWithHandle (Variables|Default|GetDashEffect))
  (Utilities|FlowControl|Delay 0.2)
  (Variables|/Script/Engine.CharacterMovementComponent|SetbIgnoreClientMovementErrorChecksAndCorrection (Variables|Default|GetMoveComponent) false)
  (Ability|EndAbility))

(event Ability|EventOnEndAbility
  (params (bWasCancelled :type Boolean)))