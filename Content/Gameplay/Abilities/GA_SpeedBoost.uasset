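; GA_SpeedBoost is a gameplay ability that applies the GE_SpeedBoost effect to its owner and stores the effect handle.
; It then runs two parallel tag-removal waits on the owning actor.
; Losing Effects.SpeedBoost prints a debug message and ends the ability.
; Losing Effects.HoldingFlower, when the flower is dropped, removes the stored effect and ends the ability, cutting the boost short.
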(event Ability|EventActivateAbility
  (bind _returnvalue (Ability|ApplyGameplayEffectToOwner "/Game/Gameplay/Effects/GE_SpeedBoost.GE_SpeedBoost_C"))
  (Variables|Default|SetOwnedEffect _returnvalue)
  (Utilities|FlowControl|Sequence
    (:then_0
      ;[1 0 0] Wait For Ability Complete
      (Ability|Tasks|WaitGameplayTagRemove "(TagName=\"Effects.SpeedBoost\")" (Ability|GetOwningActorfromActorInfo)
        (:Removed
          ;[0 1 0.05067] On Ability Complete
          (Development|PrintString "Server Removed")
          (Ability|EndAbility))))
    (:then_1
      ;[0 1 0.7847] Wait for FlowerDropped
      (Ability|Tasks|WaitGameplayTagRemove "(TagName=\"Effects.HoldingFlower\")" (Ability|GetOwningActorfromActorInfo)
        (:Removed
          ;[1 0 0.482] On Flower Dropped
          (Ability|RemoveGameplayEffectFromOwnerWithHandle (Variables|Default|GetOwnedEffect))
          (Ability|EndAbility))))))