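; Gameplay ability that makes the third-person character drop a held collectible, a flower going by the asset name.
; On activation it walks HeldCollectibles, calling TryDrop and shifting each valid item 100 units down until one drop succeeds.
; Indices of the dropped item and any invalid entries encountered are removed in reverse order by the RemoveIndices macro, then the ability ends.
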(event Ability|EventActivateAbility
  (bind _removals (Variables|Default|GetRemovals))
  (bind _asbp_third_person_character (Utilities|Casting|CastToBP_ThirdPersonCharacter (.avataractor (Ability|GetActorInfo))))
  (bind (_array_element _array_index) (Utilities|Array|ForEachLoopwithBreak (Variables|/Script/Mary.MaryCharacter|GetHeldCollectibles _asbp_third_person_character) :!label _label)
    (:LoopBody
      (Utilities|IsValid _array_element
        (:Is%20Valid
          (bind _returnvalue (Class|MaryCollectible|TryDrop _array_element))
          (Transformation|AddActorWorldOffset _array_element "0.000000,0.000000,-100.000000")
          (if _returnvalue
            (Utilities|Array|Add (Variables|Default|GetRemovals) _array_index)
            (goto _label Break)))
        (:Is%20Not%20Valid
          (Utilities|Array|Add _removals _array_index))))
    (:Completed
      (|RemoveIndices _removals (Variables|/Script/Mary.MaryCharacter|GetHeldCollectibles _asbp_third_person_character)
        (:Completed
          (Ability|EndAbility))))))