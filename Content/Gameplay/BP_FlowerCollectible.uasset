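; BP_FlowerCollectible is a collectible flower actor that grows and then blooms in the level.
; On BeginPlay the server alone starts GrowFlower with a randomized duration, drawn from a range whose bounds are themselves random.
; GrowFlower waits out that duration plus a short extra delay, calls BloomFlower and, if it succeeds, plays a pop sound at the flower's location.
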(event Custom|GrowFlower
  (params (Duration :type Float%20%28single-precision%29))
  (Utilities|FlowControl|Delay Duration)
  (Utilities|FlowControl|Delay 0.2)
  (bind _returnvalue (Class|MaryCollectible|BloomFlower))
  (if _returnvalue
    ;[1 0.3649 0.2752] MATT AND LUKE: Bloom SFX and VFX for post change
    (Audio|PlaySoundatLocation "/Game/Audio/Cues/Pop.Pop" (Transformation|GetActorLocation) "0, 0, 0" 1.0 1.0 0.0 0 0 0 0)))

(event EventBeginPlay
  (Networking|SwitchHasAuthority
    (:Authority
      (CallFunction|GrowFlower (Math|Random|RandomFloatinRange (Math|Random|RandomFloatinRange 2.0 5.0) (Math|Random|RandomFloatinRange 7.0 15.0))))))

(fn ConstructionScript)