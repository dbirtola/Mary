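; A test pickup actor that awards a point to a Mary character that overlaps its sphere.
; The server adds to the player state's points stat only while the game state's current segment is Play.
; The explosion effect and self-destruction follow outside the authority check, but a failed game state cast or a non-Play segment affects only the scoring branch.
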(event OnComponentBeginOverlap(Sphere)
  (params (OverlappedComponent :type Primitive%20Component%20Object%20Reference) (OtherActor :type Actor%20Object%20Reference) (OtherComp :type Primitive%20Component%20Object%20Reference) (OtherBodyIndex :type Integer) (bFromSweep :type Boolean) (SweepResult :type Hit%20Result%20Structure%20%28by%20ref%29))
  (bind _asmary_character (Utilities|Casting|CastToMaryCharacter OtherActor))
  (bind _asmary_player_state (Utilities|Casting|CastToMaryPlayerState (Variables|/Script/Engine.Pawn|GetPlayerState _asmary_character)))
  (Utilities|FlowControl|Sequence
    (:then_0
      (Networking|SwitchHasAuthority
        (:Authority
          (bind _asbp_mary_game_state (Utilities|Casting|CastToBP_MaryGameState (Game|GetGameState)))
          (if (Utilities|Enum|Equal(Enum) (Variables|/Script/Mary.MaryGameState|GetCurrentSegment _asbp_mary_game_state) "Play")
            (Class|MaryPlayerState|AddPlayerStat _asmary_player_state "(TagName=\"Stats.Points\")" 1.0)))))
    (:then_1
      (Effects|SpawnEmitteratLocation "/Game/StarterContent/Particles/P_Explosion.P_Explosion" (Transformation|GetActorLocation) "0, 0, 0" "2.000000,2.000000,2.000000")
      (Actor|DestroyActor))))

(fn ConstructionScript)