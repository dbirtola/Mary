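; BP_DizzySmoke is a smoke cloud that makes third-person characters dizzy, sparing its owning character.
; It spawns a pollen particle effect on BeginPlay, then enables query collision on its cylinder after a short delay.
; A capsule overlap from another character applies GE_Dizzy through that character's PlayerState ability system, with a random SetByCaller magnitude on the Data.Dizzy tag.
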(event OnComponentBeginOverlap(Cylinder)
  (params (OverlappedComponent :type Primitive%20Component%20Object%20Reference) (OtherActor :type Actor%20Object%20Reference) (OtherComp :type Primitive%20Component%20Object%20Reference) (OtherBodyIndex :type Integer) (bFromSweep :type Boolean) (SweepResult :type Hit%20Result%20Structure%20%28by%20ref%29))
  (bind _asbp_third_person_character (Utilities|Casting|CastToBP_ThirdPersonCharacter OtherActor))
  (if (and (!= _asbp_third_person_character (Variables|Default|GetOwningCharacter)) (== (Variables|/Script/Engine.Character|GetCapsuleComponent _asbp_third_person_character) OtherComp))
    (CallFunction|ApplyDIzzyEffect (Ability|GetAbilitySystemComponent (Variables|/Script/Engine.Pawn|GetPlayerState _asbp_third_person_character)))))

(event EventBeginPlay
  (Effects|SpawnEmitteratLocation "/Game/VFX/Combat_FX/Example_Smoke/P_Pollen_Temp.P_Pollen_Temp" (Transformation|GetActorLocation) "0, 0, 0" "0.500000,0.500000,0.500000")
  (Utilities|FlowControl|Delay 0.3)
  (Collision|SetCollisionEnabled (Variables|Default|GetCylinder) "QueryOnly"))

(fn ConstructionScript)

(fn ApplyDIzzyEffect
  (params (Target :type Ability%20System%20Component%20Object%20Reference))
  (bind _returnvalue (Ability|GameplayEffect|AssignTagSetbyCallerMagnitude (GameplayEffects|MakeOutgoingSpec :self Target :GameplayEffectClass "/Game/Gameplay/Effects/GE_Dizzy.GE_Dizzy_C") "(TagName=\"Data.Dizzy\")" (Math|Random|RandomFloatinRange 85.0 275.0)))
  (GameplayEffects|ApplyGameplayEffectSpecToSelf Target _returnvalue))