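; BP_MaryGameMode is a game mode that names joining players and can auto-connect non-dedicated instances to a remote server.
; On PostLogin it combines random words from two lists, retrying a bounded number of times for a name unique among player states, else setting an empty one.
; On BeginPlay, if AutoConnect is on and this is not a dedicated server, it runs a connect console command to a hardcoded IP, intended for packaged builds.
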(event EventBeginPlay
  ;[1 1 1] If we are not the server, possibly auto connect to the server. Toggle this to on before creating a packaged build to distribute. Keep it off otherwise. Please do not check this in with Auto Connect set to On.
  (Development|PrintString "Mary Game Mode determining auto connect:")
  (if (and (Variables|Default|GetAutoConnect) (not (Networking|IsDedicatedServer)))
    (Development|PrintString "Auto Connect Enabled: Attempting to auto connect to server")
    (Development|ExecuteConsoleCommand "connect 54.215.32.42" (Game|GetPlayerController 0))
    (else
      (Development|PrintString "Auto Connect Disabled:  Will not connect."))))

(event EventPostLogin
  (params (NewPlayer :type Player%20Controller%20Object%20Reference))
  (bind _player_name (CallFunction|GeneratePlayerName))
  (Class|MaryGameMode|SetPlayerName NewPlayer _player_name))

(fn ConstructionScript)

(fn GeneratePlayerName
  ;[1 1 1] If we cant get a unique name in 30 tries, dip.
  (for _index (range 0 30)
    (bind _output_get (LocalVariables|SetCurrent%20Player%20Name (Utilities|String|Append (.OutItem (Utilities|Array|Random (Variables|Default|GetName%20First%20Words))) " " (.OutItem (Utilities|Array|Random (Variables|Default|GetName%20Second%20Words))))))
    (bind _is_unique (CallFunction|IsPlayerNameUnique _output_get))
    (if _is_unique
      (return (LocalVariables|GetCurrent%20Player%20Name))))
  (return ""))

(fn IsPlayerNameUnique
  (params (Name :type String))
  (for _index (range 0 (- (Class|GameplayStatics|GetNumPlayerStates) 1))
    (if (Utilities|Enum|Equal(Enum) (PlayerState|GetPlayerName (Game|GetPlayerState _index)) Name)
      (return false)))
  (return true))