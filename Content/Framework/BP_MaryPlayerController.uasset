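; Player controller that creates the HUD and turns jump input into a dash ability.
; On BeginPlay it adds UI_HUD to the viewport, except on dedicated servers.
; IA_Jump activates GA_Dash through the Ability System Component obtained from the PlayerState, with remote activation allowed.
; Enhanced Input nodes for adding IMC_Default are present but disconnected, so this controller does not add that mapping context.
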(event Input|EnhancedActionEvents|EnhancedInputActionIA_Jump
  (params (ActionValue :type Boolean) (ElapsedSeconds :type Float%20%28double-precision%29) (TriggeredSeconds :type Float%20%28double-precision%29) (InputAction :type Input%20Action%20Object%20Reference :default "/Game/ThirdPerson/Input/Actions/IA_Jump.IA_Jump"))
  (:Triggered
    (Abilities|TryActivateAbilitybyClass (Ability|GetAbilitySystemComponent (Variables|Default|GetPlayerState)) "/Game/Gameplay/Abilities/GA_Dash.GA_Dash_C" true)))

(event EventBeginPlay
  (if (not (Networking|IsDedicatedServer))
    (bind _returnvalue (UserInterface|CreateWidget "/Game/UI/UI_HUD.UI_HUD_C"))
    (UserInterface|Viewport|AddtoViewport _returnvalue 0)))

(event EventTick
  (params (DeltaSeconds :type Float%20%28single-precision%29)))

(fn ConstructionScript)